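; BP_PlayerController is a player controller that lets a local player join the game on demand by pressing Join.
; On the first release of the Join input, it finds the PlayerStart whose tag matches the controller's ID.
; It spawns a RespawnSedan at that transform and possesses it, with a HasJoined flag preventing repeat joins.
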(event EventBeginPlay)

(event EventTick
  (params (DeltaSeconds :type Float%20%28single-precision%29)))

(event Input|ActionEvents|InputActionJoin
  (params (Key :type Key%20Structure :default "None"))
  (bind _self self)
  (bind _returnvalue (Class|GameplayStatics|GetPlayerControllerID _self))
  (:Released
    (if (not (Variables|Default|GethasJoined))
      (Variables|Default|SethasJoined true)
      (Development|PrintString (Utilities|String|ToString(Integer) _returnvalue))
      (bind _outactors (Actor|GetAllActorsOfClass "/Script/Engine.PlayerStart"))
      (for _array_element _outactors
        (if (Utilities|Name|Equal(Name) (Variables|/Script/Engine.PlayerStart|GetPlayerStartTag _array_element) (Utilities|String|StringToName (Utilities|String|ToString(Integer) _returnvalue)))
          (bind _returnvalue_2 (Game|SpawnActorfromClass "/Game/Blueprints/Nick/RespawnSedan.RespawnSedan_C" (Transformation|GetActorTransform _array_element) "Undefined" 0 0))
          (Pawn|Possess self _returnvalue_2))))))

(fn ConstructionScript)