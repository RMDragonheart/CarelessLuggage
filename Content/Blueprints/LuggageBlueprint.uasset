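; Luggage actor Blueprint that gives each instance a randomly chosen static mesh variant.
; The Construction Script uses a random, non-looping MultiGate to pick one of six branches.
; Each branch adds a static mesh component and attaches it to the Box component with relative transforms.
; The event graph holds no gameplay logic, only empty event stubs.
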(event OnComponentDeactivated(DefaultSceneRoot)
  (params (Component :type Actor%20Component%20Object%20Reference)))

(event EventBeginPlay)

(event Collision|EventActorBeginOverlap
  (params (OtherActor :type Actor%20Object%20Reference)))

(event EventTick
  (params (DeltaSeconds :type Float%20%28single-precision%29)))

(fn ConstructionScript
  (bind _box (Variables|Default|GetBox))
  (Utilities|FlowControl|MultiGate true false -1
    (:Out%200
      (bind _returnvalue (AddComponent|AddStaticMeshComponent false))
      (Transformation|AttachComponentToComponent _returnvalue _box "None" "KeepRelative" "KeepRelative" "KeepRelative" false))
    (:Out%201
      (bind _returnvalue_2 (AddComponent|AddStaticMeshComponent false))
      (Transformation|AttachComponentToComponent _returnvalue_2 _box "None" "KeepRelative" "KeepRelative" "KeepRelative" false))
    (:Out%202
      (bind _returnvalue_3 (AddComponent|AddStaticMeshComponent false))
      (Transformation|AttachComponentToComponent _returnvalue_3 _box "None" "KeepRelative" "KeepRelative" "KeepRelative" false))
    (:Out%203
      (bind _returnvalue_4 (AddComponent|AddStaticMeshComponent false))
      (Transformation|AttachComponentToComponent _returnvalue_4 _box "None" "KeepRelative" "KeepRelative" "KeepRelative" false))
    (:Out%204
      (bind _returnvalue_5 (AddComponent|AddStaticMeshComponent false))
      (Transformation|AttachComponentToComponent _returnvalue_5 _box "None" "KeepRelative" "KeepRelative" "KeepRelative" false))
    (:Out%205
      (bind _returnvalue_6 (AddComponent|AddStaticMeshComponent false))
      (Transformation|AttachComponentToComponent _returnvalue_6 _box "None" "KeepRelative" "KeepRelative" "KeepRelative" false))))